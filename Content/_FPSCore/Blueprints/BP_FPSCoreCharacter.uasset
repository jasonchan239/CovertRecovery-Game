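; BP_FPSCoreCharacter is the FPS player character Blueprint, handling the HUD and the count of remaining enemy drones.
; On BeginPlay it creates the W_Hud widget, stores a reference to it and counts all BP_EnemyAi actors to set the DronesLeft text.
; DroneDied decrements that count and refreshes the text.
; Tab calls the HUD's TABEvent to show or hide info.
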(event `self.ReceiveBeginPlay`
  ;[1 1 1] This part Creates our Widget or "HUD"
  (bind _returnvalue (`|CreateWidget` "/Game/_FPSCore/UMG/W_Hud.W_Hud_C" (`GameplayStatics.GetPlayerController` 0)))
  ;[1 1 1] This Adds it
  (`UserWidget.AddToViewport` _returnvalue 0)
  ;[1 1 1] Were using this as a reference for future calls to and from the Widget
  (set `self.HudRef` _returnvalue)
  (bind _outactors (`GameplayStatics.GetAllActorsOfClass` "/Game/Enemies/BP_EnemyAi.BP_EnemyAi_C"))
  (bind _returnvalue_2 (`KismetArrayLibrary.Array_Length` _outactors))
  (set `self.NumDrones` _returnvalue_2)
  (`TextBlock.SetText` (`/Game/_FPSCore/UMG/W_Hud.DronesLeft` (`self.HudRef`)) (`KismetTextLibrary.Conv_IntToText` _returnvalue_2)))

(event `Key|Tab`
  (params (Key :type "Key Structure"))
  ;[1 1 1] This toggles our "Show / Hide " Info
  (:`Pressed`
    (`/Game/_FPSCore/UMG/W_Hud.TAB Event` (`self.HudRef`))))

(fn `DroneDied`
  (bind _result (`/Engine/EditorBlueprintResources/StandardMacros.DecrementInt` (`self.NumDrones`))
    (:`  `
      (`TextBlock.SetText` (`/Game/_FPSCore/UMG/W_Hud.DronesLeft` (`self.HudRef`)) (`KismetTextLibrary.Conv_IntToText` _result)))))

(fn `UserConstructionScript`)