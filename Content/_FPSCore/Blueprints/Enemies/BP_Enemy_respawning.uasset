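; BP_Enemy_respawning is an FPS enemy that takes damage and fakes respawning after death.
; AnyDamage subtracts damage from Health and calls the Death event once Health reaches zero or below.
; Death hides the Cube mesh for a short delay, then shows it and resets Health, without destroying the actor or changing its collision.
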(event `self.ReceiveAnyDamage`
  (params (Damage :type "Float (single-precision)") (DamageType :type "DamageType Object Reference") (InstigatedBy :type "Controller Object Reference") (DamageCauser :type "Actor Object Reference"))
  ;[1 1 1] This is called when the actor takes any kind of "damage"
  ;[1 1 1] Here is our Health Logic
  (bind _output_get (set `self.Health` (- (`self.Health`) Damage)))
  ;[1 1 1] This part checks if Health = 0
  (if (<= _output_get 0.0)
    ;[1 1 1] if true the custom event "Death" is called
    (`self.death`)))

(event `death`
  (bind _cube (`self.Cube`))
  ;[1 1 1] This is the "Death" custom Event
  ;[1 1 1] This part is a very "Hacky" way of respawning Enemies , basically it just makes the enemy invisible for 3 seconds set by the "delay" node
  (`SceneComponent.SetVisibility` _cube false false)
  (`KismetSystemLibrary.Delay` 3.0)
  (`SceneComponent.SetVisibility` _cube true false)
  (set `self.Health` 100.0))

(fn `UserConstructionScript`)